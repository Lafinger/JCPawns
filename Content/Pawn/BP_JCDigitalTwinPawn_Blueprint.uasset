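; Player camera pawn for a digital twin viewer, with ground pan, view-plane pan, look and zoom through Enhanced Input.
; Look drives clamped control rotation, while zoom sets a target spring arm length that Tick interpolates toward.
; Curves sampled by normalized zoom scale ground-pan and zoom speed.
; FocusViewportOnActor uses component bounds, FOV and aspect ratio to pick a framing location that Tick glides toward; FocusWithCamera is empty.
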(event `self.ReceiveBeginPlay`
  (bind (_returnvalue_roll _returnvalue_pitch _returnvalue_yaw) (`KismetMathLibrary.BreakRotator` (`self.K2_GetActorRotation`)))
  (bind _returnvalue (`GameplayStatics.GetPlayerController` 0))
  (bind _returnvalue_2 (pcsubsystem `EnhancedInputLocalPlayerSubsystem` _returnvalue))
  (`|ExecutionSequence`
    (:`then_0`
      (`/Engine/EditorBlueprintResources/StandardMacros.IsValid` _returnvalue_2
        (:`Is Valid`
          (`EnhancedInputSubsystemInterface.AddMappingContext` _returnvalue_2 "/JCPawns/Input/IMC/IMC_JCDigitalTwin_Default.IMC_JCDigitalTwin_Default" 0 (struct)))))
    (:`then_1`
      (`Controller.SetControlRotation` _returnvalue (`KismetMathLibrary.MakeRotator` 0.0 _returnvalue_pitch _returnvalue_yaw))
      (`self.K2_SetActorRotation` (struct) true))
    (:`then_2`
      (set `self.TargetSpringArmLength` (`SpringArmComponent.TargetArmLength` (`self.SpringArm`))))))

(event `self.ReceiveTick`
  (params (DeltaSeconds :type "Float (single-precision)"))
  (bind _springarm (`self.SpringArm`))
  (bind _focustargetlocation (`self.FocusTargetLocation`))
  (`|ExecutionSequence`
    (:`then_0`
      (set `SpringArmComponent.TargetArmLength` (`KismetMathLibrary.FInterpTo` (`SpringArmComponent.TargetArmLength` _springarm) (`self.TargetSpringArmLength`) DeltaSeconds (`self.LagSpeed`)) _springarm))
    (:`then_1`
      (if (!= (`self.FocusCurrentLocation`) _focustargetlocation :`ErrorTolerance` 0.05)
        (bind _output_get (set `self.FocusCurrentLocation` (`KismetMathLibrary.VInterpTo` (`self.FocusStartLocation`) _focustargetlocation DeltaSeconds 10.0)))
        (set `self.FocusStartLocation` _output_get)
        (`self.K2_SetActorLocation` (`self.FocusCurrentLocation`))))))

(event `FocusViewportOnActor`
  (params (Actor :type "Actor Object Reference"))
  (bind (_sphereposition _sphereradius) (`self.GetActorBoundingBox` Actor))
  (bind _targetlocation (`self.CalcCameraLocationWithBoundingBox` _sphereposition _sphereradius 100.0))
  (set `self.FocusTargetLocation` _targetlocation)
  (set `self.FocusStartLocation` (`self.K2_GetActorLocation`)))

(event `FocusWithCamera`
  (params (Camera :type "CameraActor Object Reference")))

(event `EnhancedInput|/JCPawns/Input/IA/IA_JCDigitalTwin_GroundMove`
  (params (ActionValue :type "Vector2D Structure") (ElapsedSeconds :type "Float (double-precision)") (TriggeredSeconds :type "Float (double-precision)") (InputAction :type "InputAction Object Reference" :default "/JCPawns/Input/IA/IA_JCDigitalTwin_GroundMove.IA_JCDigitalTwin_GroundMove"))
  (bind (_x _y) (`KismetMathLibrary.BreakVector2D` ActionValue))
  (bind _groundmovespeed (`self.GroundMoveSpeed`))
  (bind _returnvalue (`CurveFloat.GetFloatValue` (`self.GroundMoveCurve`) (`self.GetZoomFactor`)))
  (bind (_returnvalue_roll _returnvalue_pitch _returnvalue_yaw) (`KismetMathLibrary.BreakRotator` (`Controller.GetControlRotation` (`GameplayStatics.GetPlayerController` 0))))
  (bind _returnvalue_2 (`KismetMathLibrary.MakeRotator` 0.0 0.0 _returnvalue_yaw))
  (:`Triggered`
    (`|ExecutionSequence`
      (:`then_0`
        (`self.K2_AddActorLocalOffset` (* (`KismetMathLibrary.GetRightVector` _returnvalue_2) _x _groundmovespeed _returnvalue)))
      (:`then_1`
        (`self.K2_AddActorLocalOffset` (* (`KismetMathLibrary.GetForwardVector` _returnvalue_2) _y _groundmovespeed _returnvalue))))))

(event `EnhancedInput|/JCPawns/Input/IA/IA_JCDigitalTwin_ViewMove`
  (params (ActionValue :type "Vector2D Structure") (ElapsedSeconds :type "Float (double-precision)") (TriggeredSeconds :type "Float (double-precision)") (InputAction :type "InputAction Object Reference" :default "/JCPawns/Input/IA/IA_JCDigitalTwin_ViewMove.IA_JCDigitalTwin_ViewMove"))
  (bind (_x _y) (`KismetMathLibrary.BreakVector2D` ActionValue))
  (bind _viewmovespeed (`self.ViewMoveSpeed`))
  (bind _returnvalue (`Controller.GetControlRotation` (`GameplayStatics.GetPlayerController` 0)))
  (:`Triggered`
    (`|ExecutionSequence`
      (:`then_0`
        (`self.K2_AddActorLocalOffset` (* (`KismetMathLibrary.GetRightVector` _returnvalue) _x _viewmovespeed)))
      (:`then_1`
        (`self.K2_AddActorLocalOffset` (* (`KismetMathLibrary.GetUpVector` _returnvalue) _y _viewmovespeed))))))

(event `EnhancedInput|/JCPawns/Input/IA/IA_JCDigitalTwin_Look`
  (params (ActionValue :type "Vector2D Structure") (ElapsedSeconds :type "Float (double-precision)") (TriggeredSeconds :type "Float (double-precision)") (InputAction :type "InputAction Object Reference" :default "/JCPawns/Input/IA/IA_JCDigitalTwin_Look.IA_JCDigitalTwin_Look"))
  (bind (_x _y) (`KismetMathLibrary.BreakVector2D` ActionValue))
  (bind (_returnvalue_roll _returnvalue_pitch _returnvalue_yaw) (`KismetMathLibrary.BreakRotator` (`self.GetControlRotation`)))
  (bind (_x_2 _y_2) (`KismetMathLibrary.BreakVector2D` (* (`self.LookClamp`) (-1.0 -1.0))))
  (:`Triggered`
    (`Controller.SetControlRotation` (`GameplayStatics.GetPlayerController` 0) (`KismetMathLibrary.MakeRotator` _returnvalue_roll (`KismetMathLibrary.FClamp` (+ (* _returnvalue_pitch (`self.LookVerticalSpeed`)) _y) _y_2 _x_2) (+ _returnvalue_yaw (* _x (`self.LookHorizontalSpeed`)))))))

(event `EnhancedInput|/JCPawns/Input/IA/IA_JCDigitalTwin_Zoom`
  (params (ActionValue :type "Float (double-precision)") (ElapsedSeconds :type "Float (double-precision)") (TriggeredSeconds :type "Float (double-precision)") (InputAction :type "InputAction Object Reference" :default "/JCPawns/Input/IA/IA_JCDigitalTwin_Zoom.IA_JCDigitalTwin_Zoom"))
  (bind (_x _y) (`KismetMathLibrary.BreakVector2D` (`self.ZoomClamp`)))
  (:`Triggered`
    (set `self.TargetSpringArmLength` (`KismetMathLibrary.FClamp` (+ (* ActionValue (`self.ZoomSpeed`) (`CurveFloat.GetFloatValue` (`self.ZoomCurve`) (`self.GetZoomFactor`))) (`self.TargetSpringArmLength`)) _x _y))))

(fn `CalcCameraLocationWithBoundingBox`
  (params (SpherePosition :type "Vector Structure") (SphereRadius :type "Float (double-precision)") (MinRadius :type "Float (double-precision)"))
  (returns (TargetLocation :type "Vector Structure"))
  (locals (TargetRadius :type "Float (double-precision)" :default 0.0) (AspectRatio :type "Float (double-precision)") (FOVAngle :type "Float (single-precision)" :default 0.0))
  (bind (_returnvalue_x _returnvalue_y) (`KismetMathLibrary.BreakVector2D` (`WidgetLayoutLibrary.GetViewportSize`)))
  (bind _returnvalue (`GameplayStatics.GetPlayerController` 0))
  (bind _output_get (set `local.FOVAngle` (`PlayerCameraManager.GetFOVAngle` (`PlayerController.PlayerCameraManager` _returnvalue))))
  (bind _output_get_2 (set `local.AspectRatio` (/ _returnvalue_x _returnvalue_y)))
  (bind _output_get_3 (set `local.TargetRadius` (`KismetMathLibrary.FMax` SphereRadius MinRadius)))
  (return (+ SpherePosition (* (`KismetMathLibrary.GetForwardVector` (`Controller.GetControlRotation` _returnvalue)) (* (/ (* _output_get_3 _output_get_2) (`KismetMathLibrary.Tan` (`KismetMathLibrary.DegreesToRadians` (/ _output_get 2.0)))) -1.0)))))

(fn `GetActorBoundingBox`
  (params (Actor :type "Actor Object Reference"))
  (returns (SpherePosition :type "Vector Structure") (SphereRadius :type "Float (single-precision)"))
  (locals (SceneComponents :type "Array of SceneComponent Object Reference") (MaxSphereRadius :type "Float (single-precision)" :default 0.0))
  (bind _rootcomponent (`Actor.RootComponent` Actor))
  (bind _maxsphereradius (`local.MaxSphereRadius`))
  (bind _output_get (set `local.SceneComponents` (`SceneComponent.GetChildrenComponents` _rootcomponent true)))
  (`KismetArrayLibrary.Array_Add` _output_get _rootcomponent)
  (for _array_element _output_get
    (bind (_origin _boxextent _sphereradius) (`KismetSystemLibrary.GetComponentBounds` _array_element))
    (if (> _sphereradius _maxsphereradius)
      (set `local.MaxSphereRadius` _maxsphereradius)))
  (return _origin _sphereradius))

(fn `GetZoomFactor`
  (returns (Factor :type "Float (double-precision)"))
  (bind (_x _y) (`KismetMathLibrary.BreakVector2D` (`self.ZoomClamp`)))
  (return (`KismetMathLibrary.NormalizeToRange` (`SpringArmComponent.TargetArmLength` (`self.SpringArm`)) _x _y)))

(fn `UserConstructionScript`)